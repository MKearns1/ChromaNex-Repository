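; BP_Stair is a construction-script actor that lays out a grid of stair static mesh tiles, with no active runtime logic.
; It clears previous tiles, sets up a base stair mesh, then loops over Width and Length to add components spaced and scaled by PanelScale.
; Tile meshes come from StairTypes by RandomIndex, but the weighted random selection and random 90-degree yaw branches are disconnected and never run.
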(event EventBeginPlay)

(event Collision|EventActorBeginOverlap
  (params (OtherActor :type Actor%20Object%20Reference)))

(event EventTick
  (params (DeltaSeconds :type Float%20%28single-precision%29)))

(fn ConstructionScript
  (Variables|Default|SetLength 0)
  (Variables|Default|SetWidth 0)
  (Variables|Default|SetPanelScale 0.0)
  (for _array_element (Variables|Default|GetStairTiles)
    (Components|DestroyComponent _array_element))
  (Utilities|Array|Clear (Variables|Default|GetStairTiles))
  (Components|StaticMesh|SetStaticMesh (Variables|Default|GetStairs1_Plane_005) (Utilities|Array|Get(acopy) (Variables|Default|GetStairTypes)))
  (Transformation|SetRelativeScale3D (Variables|Default|GetStairs1_Plane_005) (Math|Vector|MakeVector (Variables|Default|GetPanelScale) (Variables|Default|GetPanelScale) (Variables|Default|GetPanelScale)))
  (for _index (range 0 (Variables|Default|GetWidth))
    (for _index_2 (range 0 (Variables|Default|GetLength))
      (bind _returnvalue (AddComponent|AddStaticMeshComponent false))
      (Components|StaticMesh|SetStaticMesh _returnvalue (Utilities|Array|Get(acopy) (Variables|Default|GetStairTypes) (Variables|Default|GetRandomIndex)))
      (Utilities|Array|Add (Variables|Default|GetStairTiles) _returnvalue)
      (Transformation|SetRelativeLocation _returnvalue (Math|Vector|MakeVector (* _index_2 (Variables|Default|GetPanelScale) 200) (* _index (Variables|Default|GetPanelScale) 200) 0.0) false false)
      (Transformation|SetRelativeScale3D _returnvalue (Math|Vector|MakeVector (Variables|Default|GetPanelScale) (Variables|Default|GetPanelScale) (Variables|Default|GetPanelScale))))))