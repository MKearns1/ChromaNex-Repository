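; Procedural floor actor that tiles a Length by Width grid of static mesh panels, sized by PanelScale.
; The construction script calls CreateFloor, which destroys the previously stored tiles and spawns new mesh components spaced by scale.
; Each tile picks one of three FloorTypes through successive RandomPanels probability checks and gets a random quarter-turn yaw for variety.
; An older inline copy of the generation logic remains unconnected in the construction script.
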(event EventBeginPlay)

(event Collision|EventActorBeginOverlap
  (params (OtherActor :type Actor%20Object%20Reference)))

(event EventTick
  (params (DeltaSeconds :type Float%20%28single-precision%29)))

(fn ConstructionScript
  (CallFunction|CreateFloor (Variables|Default|GetLength) (Variables|Default|GetWidth) (Variables|Default|GetPanelScale)))

(fn CreateFloor
  (params (Length :type Integer) (Width :type Integer) (PanelScale :type Float%20%28double-precision%29))
  (bind _returnvalue (Math|Conversions|ToFloat(Integer) 1))
  (bind _returnvalue_2 (Math|Random|RandomFloatinRange 0.0 _returnvalue))
  (Variables|Default|SetLength Length)
  (Variables|Default|SetWidth Width)
  (Variables|Default|SetPanelScale PanelScale)
  (for _array_element (Variables|Default|GetFloorTiles)
    (Utilities|IsValid _array_element
      (:Is%20Valid
        (Components|DestroyComponent _array_element))))
  (Utilities|Array|Clear (Variables|Default|GetFloorTiles))
  (Components|StaticMesh|SetStaticMesh (Variables|Default|GetFloor) (Utilities|Array|Get(acopy) (Variables|Default|GetFloorTypes)))
  (Transformation|SetRelativeScale3D (Variables|Default|GetFloor) (Math|Vector|MakeVector (Variables|Default|GetPanelScale) (Variables|Default|GetPanelScale) (Variables|Default|GetPanelScale)))
  (for _index (range 0 (Variables|Default|GetWidth))
    (for _index_2 (range 0 (Variables|Default|GetLength))
      (bind _returnvalue_3 (AddComponent|AddStaticMeshComponent false))
      (if (<= _returnvalue_2 (Utilities|Array|Get(acopy) (Variables|Default|GetRandomPanels)))
        (Variables|Default|SetRandomIndex 0)
        (elif (<= _returnvalue_2 (Utilities|Array|Get(acopy) (Variables|Default|GetRandomPanels) 1))
          (Variables|Default|SetRandomIndex 1)
          (else
            (Variables|Default|SetRandomIndex 2))))
      (Components|StaticMesh|SetStaticMesh _returnvalue_3 (Utilities|Array|Get(acopy) (Variables|Default|GetFloorTypes) (Variables|Default|GetRandomIndex)))
      (Utilities|Array|Add (Variables|Default|GetFloorTiles) _returnvalue_3)
      (Transformation|SetRelativeLocation _returnvalue_3 (Math|Vector|MakeVector (* _index_2 (Variables|Default|GetPanelScale) 200) (* _index (Variables|Default|GetPanelScale) 200) 0.0) false false)
      (switch int (Math|Random|RandomIntegerinRange 0 3)
        (:0
          (Variables|Default|SetRandomRotation 0.0))
        (:1
          (Variables|Default|SetRandomRotation 9e+01))
        (:2
          (Variables|Default|SetRandomRotation 1.8e+02))
        (:3
          (Variables|Default|SetRandomRotation 2.7e+02)))
      (Transformation|SetRelativeRotation _returnvalue_3 (Math|Rotator|MakeRotator 0.0 0.0 (Variables|Default|GetRandomRotation)) false false)
      (Transformation|SetRelativeScale3D _returnvalue_3 (Math|Vector|MakeVector (Variables|Default|GetPanelScale) (Variables|Default|GetPanelScale) (Variables|Default|GetPanelScale))))))