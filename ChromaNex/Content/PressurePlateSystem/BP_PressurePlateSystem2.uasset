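; Pressure plate actor that switches linked target objects on or off when the player or tagged valid objects rest on it.
; Trigger overlaps keep a count of objects, and Tick watches it to flip the activated state, light material and button sound.
; A timeline slides the plate mesh vertically, then on finishing sends Interact or Off messages to TargetObject entries through ElectronicInterface.
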(event OnComponentBeginOverlap(Trigger)
  (params (OverlappedComponent :type Primitive%20Component%20Object%20Reference) (OtherActor :type Actor%20Object%20Reference) (OtherComp :type Primitive%20Component%20Object%20Reference) (OtherBodyIndex :type Integer) (bFromSweep :type Boolean) (SweepResult :type Hit%20Result%20Structure%20%28by%20ref%29))
  (if (or (Actor|ActorHasTag OtherActor "ValidPressurePlateObject") (Actor|ActorHasTag OtherActor "Player"))
    (Math|Integer|IncrementInt (Variables|Default|GetObjectsOnButton))))

(event OnComponentEndOverlap(Trigger)
  (params (OverlappedComponent :type Primitive%20Component%20Object%20Reference) (OtherActor :type Actor%20Object%20Reference) (OtherComp :type Primitive%20Component%20Object%20Reference) (OtherBodyIndex :type Integer))
  (if (or (Actor|ActorHasTag OtherActor "ValidPressurePlateObject") (Actor|ActorHasTag OtherActor "Player"))
    (Math|Integer|DecrementInt (Variables|Default|GetObjectsOnButton))))

(event EventTick
  (params (DeltaSeconds :type Float%20%28single-precision%29))
  (bind _targetobject (Variables|Default|GetTargetObject))
  (bind _cylinder_002 (Variables|Default|GetCylinder_002))
  (bind _lights (Variables|Default|GetLights))
  (bind _returnvalue (Transformation|GetRelativeTransform _cylinder_002))
  (if (Variables|Default|GetisPressurePlateActivated)
    (if (== (Variables|Default|GetObjectsOnButton) 0)
      (Rendering|Material|SetMaterial _lights 0 "/Game/PressurePlateSystem/RedLight.RedLight")
      (Variables|Default|SetisPressurePlateActivated false)
      (Variables|Default|SetisValidObjectOnTop false)
      (Audio|PlaySoundatLocation "/Game/Audio/Buttons/sound_buttons_portal_button_up_01.sound_buttons_portal_button_up_01" "0, 0, 0" "0, 0, 0" 1.0 1.0 0.0 0 0 0 0)
      (bind _newtrack_0 (Timeline|Timeline Reverse)
        (:Update
          (if (Variables|Default|GetisValidObjectOnTop)
            _
            (else
              _))
          (Transformation|SetRelativeLocation _cylinder_002 (Math|Vector|MakeVector (.x (.location _returnvalue)) (.y (.location _returnvalue)) _newtrack_0) false false))
        (:Finished
          (if (Variables|Default|GetisValidObjectOnTop)
            (Variables|Default|SetisPressurePlateActivated true)
            (for _array_element _targetobject
              (if (Utilities|DoesObjectImplementInterface (stale _array_element_2) "/Game/Interfaces/ElectronicInterface.ElectronicInterface_C")
                (Class|ElectronicInterface|Interact(Message) _array_element)))
            (else
              (Variables|Default|SetisPressurePlateActivated false)
              (for _array_element_2 _targetobject
                (if (Utilities|DoesObjectImplementInterface _array_element_2 "/Game/Interfaces/ElectronicInterface.ElectronicInterface_C")
                  (Class|ElectronicInterface|Off(Message) _array_element_2))))))))
    (elif (> (Variables|Default|GetObjectsOnButton) 0)
      (Rendering|Material|SetMaterial _lights 0 "/Game/PressurePlateSystem/GreenLight.GreenLight")
      (Variables|Default|SetisPressurePlateActivated true)
      (Variables|Default|SetisValidObjectOnTop true)
      (Audio|PlaySoundatLocation "/Game/Audio/Buttons/sound_buttons_portal_button_down_01.sound_buttons_portal_button_down_01" "0, 0, 0" "0, 0, 0" 1.0 1.0 0.0 0 0 0 0)
      (Timeline|Timeline Play))))

(fn ConstructionScript)