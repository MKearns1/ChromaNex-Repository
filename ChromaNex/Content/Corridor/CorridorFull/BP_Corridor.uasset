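; BP_Corridor is a modular sci-fi corridor actor assembled procedurally in the construction script, with no active runtime logic.
; It repeats a fixed set of corridor meshes Length times at even spacing along negative Y, tracking the end position.
; ClosedEnd adds a BP_CorridorWall child actor at that end, and HasDoorAtEnd, checked only when closed, adds a Door child actor.
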(event EventBeginPlay)

(event Collision|EventActorBeginOverlap
  (params (OtherActor :type Actor%20Object%20Reference)))

(event EventTick
  (params (DeltaSeconds :type Float%20%28single-precision%29)))

(fn ConstructionScript
  (Variables|Default|SetCorridorObjects (Utilities|Array|MakeArray (Variables|Default|GetSci_Fi_Corridor_Bolts_2) (Variables|Default|GetSci_Fi_Corridor_Other) (Variables|Default|GetSci_Fi_Corridor_Other_2) (Variables|Default|GetSci_Fi_Corridor_Bolts) (Variables|Default|GetSci_Fi_Corridor_Pipes) (Variables|Default|GetSci_Fi_Corridor_Corridor) (Variables|Default|GetSci_Fi_Corridor_Cylinders) (Variables|Default|GetSci_Fi_Corridor_Floor)))
  (for _index (range 0 (Variables|Default|GetLength))
    (for _array_element (Variables|Default|GetCorridorObjects)
      (bind _returnvalue (AddComponent|AddStaticMeshComponent false))
      (Components|StaticMesh|SetStaticMesh _returnvalue (Variables|/Script/Engine.StaticMeshComponent|GetStaticMesh _array_element))
      (Transformation|SetRelativeLocation _returnvalue (Math|Vector|MakeVector 0.0 (Math|Conversions|ToFloat(Integer) (* _index -1050)) 0.0) false false)
      (Variables|Default|SetEndPosition (Math|Vector|MakeVector 0.0 (+ (Math|Conversions|ToFloat(Integer) (* _index -1050)) -1.05e+03) 0.0))))
  (if (Variables|Default|GetClosedEnd)
    (bind _returnvalue_2 (AddComponent|AddChildActorComponent false))
    (ChildActorComponent|SetChildActorClass _returnvalue_2 "/Game/Corridor/CorridorWall/BP_CorridorWall.BP_CorridorWall_C")
    (bind _output_get (Variables|Default|SetOffset "-637.764566,800.000000,0.000000"))
    (Transformation|SetRelativeLocation _returnvalue_2 (+ _output_get (Variables|Default|GetEndPosition)) false false)
    (Transformation|SetRelativeRotation _returnvalue_2 "0.000000,90.000000,0.000000" false false)
    (Transformation|SetRelativeScale3D _returnvalue_2 "1.000000,1.250000,1.000000")
    (if (Variables|Default|GetHasDoorAtEnd)
      (bind _returnvalue_3 (AddComponent|AddChildActorComponent false))
      (ChildActorComponent|SetChildActorClass _returnvalue_3 "/Game/DoorSystem/Door.Door_C")
      (bind _output_get_2 (Variables|Default|SetOffset "-0.000000,250.000000,0.000000"))
      (Transformation|SetRelativeLocation _returnvalue_3 (+ _output_get_2 (Variables|Default|GetEndPosition)) false false)
      (Transformation|SetRelativeRotation _returnvalue_3 "0.000000,0.000000,0.000000" false false)
      (Transformation|SetRelativeScale3D _returnvalue_3 "2.500000,2.000000,2.500000"))))