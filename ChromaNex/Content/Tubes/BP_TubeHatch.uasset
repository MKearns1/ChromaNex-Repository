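; BP_TubeHatch is an interactable tube hatch that dispenses a BP_Cube, destroying the previously dispensed one.
; A timeline swings two doors open and switches the light material, then spawns the cube at CubeSpawnPoint.
; While open, Tick drives the cube's physics velocity toward CubeDestination.
; The cube overlapping Trigger reverses the timeline to close the hatch, halving its velocity unless CarryMomentum is set.
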(event OnComponentBeginOverlap(Trigger)
  (params (OverlappedComponent :type Primitive%20Component%20Object%20Reference) (OtherActor :type Actor%20Object%20Reference) (OtherComp :type Primitive%20Component%20Object%20Reference) (OtherBodyIndex :type Integer) (bFromSweep :type Boolean) (SweepResult :type Hit%20Result%20Structure%20%28by%20ref%29))
  (bind _currentcube (Variables|Default|GetCurrentCube))
  (bind _staticmesh (Variables|/Game/Cube/BP_Cube.BP_Cube_C|GetStaticMesh _currentcube))
  (if (== OtherActor (Variables|Default|GetCurrentCube))
    (CallFunction|CloseHatch)
    (if (not (Variables|Default|GetCarryMomentum))
      (Utilities|IsValid _currentcube
        (:Is%20Valid
          (Utilities|IsValid _staticmesh
            (:Is%20Valid
              (bind _returnvalue (Physics|GetPhysicsLinearVelocity _staticmesh "None"))
              (Physics|SetPhysicsLinearVelocity _staticmesh (* _returnvalue 0.5) false "None"))))))))

(event Custom|OpenHatch
  (bind _currentcube (Variables|Default|GetCurrentCube))
  (if (not (Variables|Default|GetOpen))
    (Variables|Default|SetOpen true)
    (Utilities|IsValid _currentcube
      (:Is%20Valid
        (Default|DestroySelf _currentcube))
      (:Is%20Not%20Valid
        _))
    (Audio|PlaySoundatLocation (Variables|Default|GetSound1) (Transformation|GetWorldLocation (Variables|Default|GetDefaultSceneRoot)) "0, 0, 0" 1.0 1.0 0.0 0 0 0 0)
    (Rendering|Material|SetMaterial (Variables|Default|GetTubeHatch_Cube_001) 2 "/Game/Tubes/HatchLight_Mat_Open.HatchLight_Mat_Open")
    (bind _rotation (Timeline|Timeline Play)
      (:Update
        (Transformation|SetRelativeRotation (Variables|Default|GetHatchPivot2) (Math|Rotator|MakeRotator 0.0 (Math|Float|Lerp 0.0 -9e+01 _rotation) 0.0) false false)
        (Transformation|SetRelativeRotation (Variables|Default|GetHatchPivot1) (Math|Rotator|MakeRotator 0.0 (* (Math|Float|Lerp 0.0 -9e+01 _rotation) -1.0) 0.0) false false))
      (:Finished
        (if (Variables|Default|GetOpen)
          (CallFunction|SpawnCube)
          (else
            (Rendering|Material|SetMaterial (Variables|Default|GetTubeHatch_Cube_001) 2 "/Game/Tubes/HatchLight_Mat_Default.HatchLight_Mat_Default")))))))

(event Custom|CloseHatch
  (Variables|Default|SetOpen false)
  (bind _rotation (Timeline|Timeline Reverse)
    (:Update
      (Transformation|SetRelativeRotation (Variables|Default|GetHatchPivot2) (Math|Rotator|MakeRotator 0.0 (Math|Float|Lerp 0.0 -9e+01 _rotation) 0.0) false false)
      (Transformation|SetRelativeRotation (Variables|Default|GetHatchPivot1) (Math|Rotator|MakeRotator 0.0 (* (Math|Float|Lerp 0.0 -9e+01 _rotation) -1.0) 0.0) false false))
    (:Finished
      (if (Variables|Default|GetOpen)
        (CallFunction|SpawnCube)
        (else
          (Rendering|Material|SetMaterial (Variables|Default|GetTubeHatch_Cube_001) 2 "/Game/Tubes/HatchLight_Mat_Default.HatchLight_Mat_Default"))))))

(event Custom|SpawnCube
  (bind _returnvalue (Game|SpawnActorfromClass "/Game/Cube/BP_Cube.BP_Cube_C" (Transformation|GetWorldTransform (Variables|Default|GetCubeSpawnPoint)) "Undefined" "MultiplyWithRoot" 0 0))
  (bind _output_get (Variables|Default|SetCurrentCube _returnvalue))
  (Variables|Default|SetMovementDirection (Math|Vector|Normalize (- (Transformation|GetWorldLocation (Variables|Default|GetCube%20Destination)) (Transformation|GetWorldLocation (Variables|/Game/Cube/BP_Cube.BP_Cube_C|GetDefaultSceneRoot _output_get))) 1.0)))

(event Custom|DispenseCube
  (CallFunction|OpenHatch))

(event EventBeginPlay)

(event Collision|EventActorBeginOverlap
  (params (OtherActor :type Actor%20Object%20Reference)))

(event EventTick
  (params (DeltaSeconds :type Float%20%28single-precision%29))
  (bind _currentcube (Variables|Default|GetCurrentCube))
  (bind _staticmesh (Variables|/Game/Cube/BP_Cube.BP_Cube_C|GetStaticMesh _currentcube))
  (if (Variables|Default|GetOpen)
    (Utilities|IsValid _currentcube
      (:Is%20Valid
        (Utilities|IsValid _staticmesh
          (:Is%20Valid
            (Physics|SetPhysicsLinearVelocity _staticmesh (* (Variables|Default|GetMovementDirection) (Variables|Default|GetCubeSpeed)) false "None")))))))

(event EventInteract
  (CallFunction|DispenseCube))

(fn ConstructionScript
  (Components|Timeline|SetPlayRate (Variables|Default|GetTimeline) (Variables|Default|GetHatchSpeed)))