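; BP_PedestalButton is a pressable pedestal button that switches linked electronic objects on, then resets itself after a delay.
; Interact calls PressButton, which turns the light green and runs a Timeline that moves the button's Z.
; On finish, TargetObject entries implementing ElectronicInterface receive InteractMessage, and a delay leads to RaiseButton.
; RaiseButton restores red and reverses the same Timeline, whose Finished branch then sends OffMessage because OnOff is false.
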(event OnComponentBeginOverlap(Trigger)
  (params (OverlappedComponent :type Primitive%20Component%20Object%20Reference) (OtherActor :type Actor%20Object%20Reference) (OtherComp :type Primitive%20Component%20Object%20Reference) (OtherBodyIndex :type Integer) (bFromSweep :type Boolean) (SweepResult :type Hit%20Result%20Structure%20%28by%20ref%29)))

(event OnComponentEndOverlap(Trigger)
  (params (OverlappedComponent :type Primitive%20Component%20Object%20Reference) (OtherActor :type Actor%20Object%20Reference) (OtherComp :type Primitive%20Component%20Object%20Reference) (OtherBodyIndex :type Integer)))

(event Custom|PressButton
  (bind _pedestalbutton_button (Variables|Default|GetPedestalButton_Button))
  (bind _returnvalue (Transformation|GetRelativeTransform _pedestalbutton_button))
  (if (not (Variables|Default|GetOn/Off))
    (Variables|Default|SetOn/Off true)
    (Rendering|Material|SetMaterial (Variables|Default|GetPedestalButton_Cylinder_006) 0 "/Game/PressurePlateSystem/GreenLight.GreenLight")
    (bind _newtrack_0 (Timeline|Timeline Play)
      (:Update
        (Transformation|SetRelativeLocation _pedestalbutton_button (Math|Vector|MakeVector (.x (.location _returnvalue)) (.y (.location _returnvalue)) _newtrack_0) false false))
      (:Finished
        (for _array_element (Variables|Default|GetTargetObject)
          (if (Utilities|DoesObjectImplementInterface _array_element "/Game/Interfaces/ElectronicInterface.ElectronicInterface_C")
            (if (Variables|Default|GetOn/Off)
              (Class|ElectronicInterface|Interact(Message) _array_element)
              (Utilities|FlowControl|Delay (Variables|Default|GetTime%20Between%20Presses))
              (Variables|Default|SetOn/Off false)
              (CallFunction|RaiseButton)
              (else
                (Class|ElectronicInterface|Off(Message) _array_element)))))))))

(event Custom|RaiseButton
  (bind _pedestalbutton_button (Variables|Default|GetPedestalButton_Button))
  (bind _returnvalue (Transformation|GetRelativeTransform _pedestalbutton_button))
  (Variables|Default|SetOn/Off false)
  (Rendering|Material|SetMaterial (Variables|Default|GetPedestalButton_Lights) 0 "/Game/PressurePlateSystem/RedLight.RedLight")
  (bind _newtrack_0 (Timeline|Timeline Reverse)
    (:Update
      (Transformation|SetRelativeLocation _pedestalbutton_button (Math|Vector|MakeVector (.x (.location _returnvalue)) (.y (.location _returnvalue)) _newtrack_0) false false))
    (:Finished
      (for _array_element (Variables|Default|GetTargetObject)
        (if (Utilities|DoesObjectImplementInterface _array_element "/Game/Interfaces/ElectronicInterface.ElectronicInterface_C")
          (if (Variables|Default|GetOn/Off)
            (Class|ElectronicInterface|Interact(Message) _array_element)
            (Utilities|FlowControl|Delay (Variables|Default|GetTime%20Between%20Presses))
            (Variables|Default|SetOn/Off false)
            (CallFunction|RaiseButton)
            (else
              (Class|ElectronicInterface|Off(Message) _array_element))))))))

(event EventBeginPlay)

(event Collision|EventActorBeginOverlap
  (params (OtherActor :type Actor%20Object%20Reference)))

(event EventTick
  (params (DeltaSeconds :type Float%20%28single-precision%29)))

(event EventInteract
  (params (Player :type BP%20First%20Person%20Character%20Object%20Reference) (HitComponent :type Primitive%20Component%20Object%20Reference) (Location :type Vector :default "0, 0, 0"))
  (CallFunction|PressButton))

(fn ConstructionScript)