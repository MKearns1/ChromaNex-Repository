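; Test modular block actor whose construction script fits a box body and edge pieces between eight corner components.
; It centres the Cube on the average corner position and scales it from offsets between corners.
; Five middle edge meshes are stretched along X from corner spacing and placed at corners, some mirrored in Z.
; An older grid-spawning loop is left disconnected, and the event graph is empty.
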(event EventBeginPlay)

(event Collision|EventActorBeginOverlap
  (params (OtherActor :type Actor%20Object%20Reference)))

(event EventTick
  (params (DeltaSeconds :type Float%20%28single-precision%29)))

(fn ConstructionScript
  (Variables|Default|SetCentrePosition (/ (+ (Variables|/Script/Engine.SceneComponent|GetRelativeLocation (Variables|Default|GetModularBlockCorner)) (Variables|/Script/Engine.SceneComponent|GetRelativeLocation (Variables|Default|GetModularBlockCorner1)) (Variables|/Script/Engine.SceneComponent|GetRelativeLocation (Variables|Default|GetModularBlockCorner2)) (Variables|/Script/Engine.SceneComponent|GetRelativeLocation (Variables|Default|GetModularBlockCorner3)) (Variables|/Script/Engine.SceneComponent|GetRelativeLocation (Variables|Default|GetModularBlockCorner4)) (Variables|/Script/Engine.SceneComponent|GetRelativeLocation (Variables|Default|GetModularBlockCorner5)) (Variables|/Script/Engine.SceneComponent|GetRelativeLocation (Variables|Default|GetModularBlockCorner6)) (Variables|/Script/Engine.SceneComponent|GetRelativeLocation (Variables|Default|GetModularBlockCorner7))) 8.0))
  (Transformation|SetRelativeLocation (Variables|Default|GetCube) (Variables|Default|GetCentrePosition) false false)
  (CallFunction|CalculateBodyDimensions)
  (Transformation|SetRelativeScale3D (Variables|Default|GetCube) (Variables|Default|GetBodyScale))
  (CallFunction|CalculateEdgeDimensions))

(fn CalculateBodyDimensions
  (Variables|Default|SetBodyScale (Math|Vector|MakeVector (/ (.x (- (+ (Variables|/Script/Engine.SceneComponent|GetRelativeLocation (Variables|Default|GetModularBlockCorner3)) "-100.000000,0.000000,0.000000") (Variables|/Script/Engine.SceneComponent|GetRelativeLocation (Variables|Default|GetModularBlockCorner2)))) 1e+02) (/ (.y (- (Variables|/Script/Engine.SceneComponent|GetRelativeLocation (Variables|Default|GetModularBlockCorner2)) (Variables|/Script/Engine.SceneComponent|GetRelativeLocation (Variables|Default|GetModularBlockCorner1)))) 1e+02) (/ (.z (- (+ (Variables|/Script/Engine.SceneComponent|GetRelativeLocation (Variables|Default|GetModularBlockCorner4)) "0.000000,0.000000,-50.000000") (Variables|/Script/Engine.SceneComponent|GetRelativeLocation (Variables|Default|GetModularBlockCorner2)))) 1e+02))))

(fn CalculateEdgeDimensions
  (bind _modularblockmiddle (Variables|Default|GetModularBlockMiddle))
  (Transformation|SetRelativeScale3D _modularblockmiddle (Math|Vector|MakeVector (/ (.x (- (+ (Variables|/Script/Engine.SceneComponent|GetRelativeLocation (Variables|Default|GetModularBlockCorner3)) "0.000000,0.000000,0.000000") (Variables|/Script/Engine.SceneComponent|GetRelativeLocation (Variables|Default|GetModularBlockCorner2)))) 5e+01) 1.0 1.0))
  (Transformation|SetRelativeLocation _modularblockmiddle (Variables|/Script/Engine.SceneComponent|GetRelativeLocation (Variables|Default|GetModularBlockCorner2)) false false)
  (Transformation|SetRelativeScale3D (Variables|Default|GetModularBlockMiddle1) (* (Variables|/Script/Engine.SceneComponent|GetRelativeScale3D (Variables|Default|GetModularBlockMiddle)) "1.000000,1.000000,-1.000000"))
  (Transformation|SetRelativeLocation (Variables|Default|GetModularBlockMiddle1) (Variables|/Script/Engine.SceneComponent|GetRelativeLocation (Variables|Default|GetModularBlockCorner4)) false false)
  (Transformation|SetRelativeScale3D (Variables|Default|GetModularBlockMiddle2) (Variables|/Script/Engine.SceneComponent|GetRelativeScale3D (Variables|Default|GetModularBlockMiddle)))
  (Transformation|SetRelativeLocation (Variables|Default|GetModularBlockMiddle2) (Variables|/Script/Engine.SceneComponent|GetRelativeLocation (Variables|Default|GetModularBlockCorner)) false false)
  (Transformation|SetRelativeScale3D (Variables|Default|GetModularBlockMiddle3) (* (Variables|/Script/Engine.SceneComponent|GetRelativeScale3D (Variables|Default|GetModularBlockMiddle)) "1.000000,1.000000,-1.000000"))
  (Transformation|SetRelativeLocation (Variables|Default|GetModularBlockMiddle3) (Variables|/Script/Engine.SceneComponent|GetRelativeLocation (Variables|Default|GetModularBlockCorner7)) false false)
  (Transformation|SetRelativeScale3D (Variables|Default|GetModularBlockMiddle4) (Math|Vector|MakeVector (/ (.y (- (+ (Variables|/Script/Engine.SceneComponent|GetRelativeLocation (Variables|Default|GetModularBlockCorner2)) "") (Variables|/Script/Engine.SceneComponent|GetRelativeLocation (Variables|Default|GetModularBlockCorner1)))) 5e+01) 1.0 1.0))
  (Transformation|SetRelativeLocation (Variables|Default|GetModularBlockMiddle4) (Variables|/Script/Engine.SceneComponent|GetRelativeLocation (Variables|Default|GetModularBlockCorner1)) false false))