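; BP_Cube is a physics cube that the player can grab through Interact using their physics handle, with a Colour option that applies a yellow material and physical material at construction.
; Impacts play a pitch-randomized sound behind speed checks and a short cooldown, ignoring the player and hits reporting the yellow physical material.
; DestroySelf breaks the cube by removing its main mesh and simulating physics on six side pieces, then destroys the actor after a delay.
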(event OnComponentHit(StaticMesh)
  (params (HitComponent :type Primitive%20Component%20Object%20Reference) (OtherActor :type Actor%20Object%20Reference) (OtherComp :type Primitive%20Component%20Object%20Reference) (NormalImpulse :type Vector :default "0, 0, 0") (Hit :type Hit%20Result%20Structure%20%28by%20ref%29))
  (bind (_bblockinghit _binitialoverlap _time _distance _location _impactpoint _normal _impactnormal _physmat) (Collision|BreakHitResult Hit))
  (if (not (== OtherActor (Game|GetPlayerCharacter 0)))
    (if (not (== _physmat "/Game/Materials/PhysicsMaterials/PM_Yellow.PM_Yellow"))
      (if (> (Math|Float|Absolute(Float) (Math|Vector|DotProduct (Transformation|GetComponentVelocity (Variables|Default|GetStaticMesh)) _impactnormal)) 2e+01)
        (CallFunction|CollisionSound)))))

(event Custom|DestroySelf
  (Components|DestroyComponent (Variables|Default|GetStaticMesh))
  (for _array_element (Variables|Default|GetSides)
    (Physics|SetSimulatePhysics _array_element true)
    (Transformation|AddRelativeRotation _array_element (* (Math|Random|RandomRotator false) 0.1) false false)
    (Collision|SetCollisionEnabled _array_element "QueryAndPhysics"))
  (Utilities|FlowControl|Delay 2.0)
  (Actor|DestroyActor))

(event Custom|CollisionSound
  (if (not (Variables|Default|GetHitASurface))
    (if (> (Math|Vector|VectorLength (Transformation|GetComponentVelocity (Variables|Default|GetStaticMesh))) 5e+01)
      (Audio|PlaySoundatLocation (Variables|Default|GetCollisionSound1) (Transformation|GetWorldLocation (Variables|Default|GetStaticMesh)) "0, 0, 0" 1.0 (Math|Random|RandomFloatinRange 0.8 2.0) 0.0 0 0 0 0)
      (Variables|Default|SetHitASurface true)
      (Utilities|FlowControl|Delay 0.5)
      (Variables|Default|SetHitASurface false))))

(event EventBeginPlay
  (Variables|Default|SetSides (Utilities|Array|MakeArray (Variables|Default|GetSide1) (Variables|Default|GetSide2) (Variables|Default|GetSide3) (Variables|Default|GetSide4) (Variables|Default|GetSide5) (Variables|Default|GetSide6))))

(event Collision|EventActorBeginOverlap
  (params (OtherActor :type Actor%20Object%20Reference)))

(event EventTick
  (params (DeltaSeconds :type Float%20%28single-precision%29)))

(event EventYellow
  (bind _staticmesh (Variables|Default|GetStaticMesh))
  (Class|PrimitiveComponent|SetPhysMaterialOverride _staticmesh "/Game/Materials/PhysicsMaterials/PM_Yellow.PM_Yellow")
  (Rendering|Material|SetMaterial _staticmesh 0 "/Game/Materials/MI_Yellow.MI_Yellow"))

(event EventDefault
  (bind _staticmesh (Variables|Default|GetStaticMesh))
  (Class|PrimitiveComponent|SetPhysMaterialOverride _staticmesh)
  (Rendering|Material|SetMaterial _staticmesh 0 "/Game/FPWeapon/Materials/BaseMaterial.BaseMaterial"))

(fn ConstructionScript
  (switch string (Variables|Default|GetColour)
    (:Yellow
      (CallFunction|Yellow))))

(fn Interact
  (params (Player :type BP%20First%20Person%20Character%20Object%20Reference) (HitComponent :type Primitive%20Component%20Object%20Reference) (Location :type Vector :default "0, 0, 0"))
  (Physics|Components|PhysicsHandle|GrabComponentatLocationwithRotation (Variables|/Game/FirstPerson/Blueprints/BP_FirstPersonCharacter.BP_FirstPersonCharacter_C|GetPhysicsHandle Player) HitComponent "None" Location "0, 0, 0")
  (return))