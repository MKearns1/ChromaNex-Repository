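; BP_SimpleDoor is a sliding door that opens on an Interact event and closes itself after a configurable delay.
; The construction script caches Side2's starting position, and a timeline lerps that panel 50 units along its relative X axis.
; OpenDoor plays the timeline and sets a timer by function name to CloseDoor, which reverses it.
; An older Open/Direction toggle using a second timeline remains disconnected and never runs.
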(event Custom|OpenDoor
  (Utilities|Time|SetTimerbyFunctionName 0 "CloseDoor" (Variables|Default|GetResetDelay))
  (bind _newtrack_0 (Timeline|Timeline_2 Play)
    (:Update
      (Transformation|SetRelativeLocation (Variables|Default|GetSide2) (Math|Vector|Lerp(Vector) (Variables|Default|GetInitialPosition) (+ (Variables|Default|GetInitialPosition) "50.000000,0.000000,0.000000") _newtrack_0) false false))))

(event Custom|CloseDoor
  (bind _newtrack_0 (Timeline|Timeline_2 Reverse)
    (:Update
      (Transformation|SetRelativeLocation (Variables|Default|GetSide2) (Math|Vector|Lerp(Vector) (Variables|Default|GetInitialPosition) (+ (Variables|Default|GetInitialPosition) "50.000000,0.000000,0.000000") _newtrack_0) false false))))

(event EventBeginPlay)

(event Collision|EventActorBeginOverlap
  (params (OtherActor :type Actor%20Object%20Reference)))

(event EventTick
  (params (DeltaSeconds :type Float%20%28single-precision%29)))

(event EventInteract
  (CallFunction|OpenDoor))

(fn ConstructionScript
  (Variables|Default|SetInitialPosition (Variables|/Script/Engine.SceneComponent|GetRelativeLocation (Variables|Default|GetSide2))))