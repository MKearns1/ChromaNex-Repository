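; Billboard actor with an old TV mesh whose LED material is chosen by its Colour variable.
; The construction script switches on Colour to apply the matching LED material to slot 1 of the TV mesh.
; Unmatched values call Default, which resets Colour to "Default" and applies black LED to both the Cube and TV mesh.
; GetColour exposes the current colour; there is no active BeginPlay, overlap or Tick logic.
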(event EventBeginPlay)

(event Collision|EventActorBeginOverlap
  (params (OtherActor :type Actor%20Object%20Reference)))

(event EventTick
  (params (DeltaSeconds :type Float%20%28single-precision%29)))

(event EventDefault
  (Variables|Default|SetColour "Default")
  (Rendering|Material|SetMaterial (Variables|Default|GetCube) 1 "/Game/Billboard/LEDBlack.LEDBlack"))

(fn ConstructionScript
  (switch string (Variables|Default|GetColour)
    (:Default
      (CallFunction|Default))
    (:Green
      (Variables|Default|SetMaterialArray "/Game/Billboard/LEDGreen.LEDGreen")
      (Rendering|Material|SetMaterial (Variables|Default|GetOld_Tvsa_tetri_tv_main_low_006) 1 (Variables|Default|GetMaterialArray) :!label _label))
    (:Yellow
      (Variables|Default|SetMaterialArray "/Game/Billboard/LEDYellow.LEDYellow")
      (goto _label))
    (:Red
      (Variables|Default|SetMaterialArray "/Game/Billboard/LEDRed.LEDRed")
      (goto _label))
    (:Purple
      (Variables|Default|SetMaterialArray "/Game/Billboard/LEDPurple.LEDPurple")
      (goto _label))
    (:Blue
      (Variables|Default|SetMaterialArray "/Game/Billboard/LEDBlue.LEDBlue")
      (goto _label))
    (:White
      (Variables|Default|SetMaterialArray "/Game/Billboard/LEDYWhite.LEDYWhite")
      (goto _label))
    (:Black
      (Variables|Default|SetMaterialArray "/Game/Billboard/LEDBlack.LEDBlack")
      (goto _label))))

(fn GetColour
  (return (Variables|Default|GetColour)))