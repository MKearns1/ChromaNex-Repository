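; BP_SetLevelColours is a level setup actor that configures the first-person player for the current level.
; On BeginPlay it casts the player character to BP_FirstPersonCharacter and copies its LevelColours into the character's ColourCharges.
; A StartWithGun flag decides whether it adds a BP weapon component to the player and sets HasGun accordingly.
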(event EventBeginPlay
  (bind _asbp_first_person_character (Utilities|Casting|CastToBP_FirstPersonCharacter (Game|GetPlayerCharacter 0)))
  (bind _output_get (Variables|Default|SetBP_Player _asbp_first_person_character))
  (Variables|/Game/FirstPerson/Blueprints/BP_FirstPersonCharacter.BP_FirstPersonCharacter_C|SetColour%20Charges _output_get (Variables|Default|GetLevel%20Colours))
  (if (Variables|Default|GetStartWithGun)
    (AddComponent|AddBPWeaponComponent (Variables|Default|GetBP_Player) false)
    (Variables|/Game/FirstPerson/Blueprints/BP_FirstPersonCharacter.BP_FirstPersonCharacter_C|SetHasGun (Variables|Default|GetBP_Player) true)
    (else
      (Variables|/Game/FirstPerson/Blueprints/BP_FirstPersonCharacter.BP_FirstPersonCharacter_C|SetHasGun (Variables|Default|GetBP_Player) false))))

(event Collision|EventActorBeginOverlap
  (params (OtherActor :type Actor%20Object%20Reference)))

(event EventTick
  (params (DeltaSeconds :type Float%20%28single-precision%29)))

(fn ConstructionScript)