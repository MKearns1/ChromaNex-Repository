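; Launch trigger that throws the first-person player character along a ballistic arc when they enter its box.
; BeginPlay precomputes launch velocity from the From-to-To offset, gravity and an apex height derived from landing rise and horizontal distance.
; Launch zeroes air control; Tick restores it whenever horizontal speed is 600 or below.
; Despite the name, the speed-threshold check is disconnected, so any player overlap launches; debug prints remain.
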(event OnComponentBeginOverlap(Box)
  (params (OverlappedComponent :type Primitive%20Component%20Object%20Reference) (OtherActor :type Actor%20Object%20Reference) (OtherComp :type Primitive%20Component%20Object%20Reference) (OtherBodyIndex :type Integer) (bFromSweep :type Boolean) (SweepResult :type Hit%20Result%20Structure%20%28by%20ref%29))
  (if (== OtherActor (Variables|Default|GetPlayer_BP))
    (Development|PrintString "Hello")
    (Character|LaunchCharacter (Variables|Default|GetPlayer_BP) (Variables|Default|GetLaunchVelocity) true true)
    (CallFunction|SetAirControl false)))

(event Custom|CalculateLaunchDirection
  (Variables|Default|SetLaunchDirection (Math|Vector|Normalize (- (Transformation|GetWorldLocation (Variables|Default|GetTo)) (Transformation|GetWorldLocation (Variables|Default|GetFrom))) 1.0)))

(event Custom|CalculateHorizontalVelocity
  (Variables|Default|SetHorizontalVelocity (/ (Variables|Default|GetHorizontalDistance) (Variables|Default|GetTimeOfFlight))))

(event Custom|CalculateLaunchVelocity
  (bind _horizontalvelocity (Variables|Default|GetHorizontalVelocity))
  (Variables|Default|SetLaunchVelocity (Math|Vector|MakeVector (.x _horizontalvelocity) (.y _horizontalvelocity) (Variables|Default|GetInitialVerticalVelocity))))

(event Custom|CalculateMaxHeight
  (Variables|Default|SetMaxHeight (+ (.z (- (Variables|Default|GetLandPoint) (Variables|Default|GetStartPoint))) (/ (Math|Vector|VectorLengthXY (Variables|Default|GetHorizontalDistance)) 4.0))))

(event Custom|SetAirControl
  (params (On/Off :type Boolean))
  (bind _player_bp (Variables|Default|GetPlayer_BP))
  (bind _charactermovement (Variables|/Script/Engine.Character|GetCharacterMovement _player_bp))
  (if On/Off
    (Variables|/Script/Engine.CharacterMovementComponent|SetAirControl _charactermovement 0.05)
    (Variables|/Script/Engine.CharacterMovementComponent|SetBrakingDecelerationFlying _charactermovement 2048.0)
    (Variables|/Script/Engine.CharacterMovementComponent|SetBrakingDecelerationFalling _charactermovement 0.0)
    (else
      (Variables|/Script/Engine.CharacterMovementComponent|SetAirControl _charactermovement 0.0)
      (Variables|/Script/Engine.CharacterMovementComponent|SetBrakingDecelerationFlying _charactermovement 0.0)
      (Variables|/Script/Engine.CharacterMovementComponent|SetBrakingDecelerationFalling _charactermovement 0.0))))

(event Custom|CalculateFlightTime
  (Variables|Default|SetTimeOfFlight (/ (* (Variables|Default|GetInitialVerticalVelocity) 2.0) (* (Components|Movement|GetGravityZ (Variables|/Script/Engine.Character|GetCharacterMovement (Variables|Default|GetPlayer_BP))) -1.0))))

(event Custom|CalculateVerticalVelocity
  ;[0 0 0] Calculate Z velocity
  (Variables|Default|SetInitialVerticalVelocity (Math|Float|Sqrt (* (* (Components|Movement|GetGravityZ (Variables|/Script/Engine.Character|GetCharacterMovement (Variables|Default|GetPlayer_BP))) -1.0) (Variables|Default|GetMaxHeight) 2.0))))

(event Custom|CalculateHorizontalDistance
  ;[0 0 0] Calculate XY Distance
  (Variables|Default|SetHorizontalDistance (- (Transformation|GetWorldLocation (Variables|Default|GetTo)) (Transformation|GetWorldLocation (Variables|Default|GetFrom)))))

(event EventBeginPlay
  (bind _asbp_first_person_character (Utilities|Casting|CastToBP_FirstPersonCharacter (Game|GetPlayerCharacter 0)))
  (Variables|Default|SetPlayer_BP _asbp_first_person_character)
  (CallFunction|CalculateLaunchDirection)
  (CallFunction|CalculateHorizontalDistance)
  (CallFunction|CalculateMaxHeight)
  (CallFunction|CalculateVerticalVelocity)
  (CallFunction|CalculateFlightTime)
  (CallFunction|CalculateHorizontalVelocity)
  (CallFunction|CalculateLaunchVelocity))

(event Collision|EventActorBeginOverlap
  (params (OtherActor :type Actor%20Object%20Reference)))

(event EventTick
  (params (DeltaSeconds :type Float%20%28single-precision%29))
  (bind _player_bp (Variables|Default|GetPlayer_BP))
  (bind _output_get (Variables|Default|SetSpeedInLaunchDirection (Math|Vector|DotProduct (Transformation|GetComponentVelocity (Variables|/Script/Engine.Character|GetCapsuleComponent (Variables|Default|GetPlayer_BP))) (Variables|Default|GetLaunchDirection))))
  (CallFunction|CalculateMaxHeight)
  (Development|PrintString (Utilities|String|ToString(Integer) (Variables|/Game/FirstPerson/Blueprints/BP_FirstPersonCharacter.BP_FirstPersonCharacter_C|GetSelectedColour _player_bp)))
  (if (<= (Math|Vector|VectorLengthXY (Variables|/Script/Engine.MovementComponent|GetVelocity (Variables|/Script/Engine.Character|GetCharacterMovement _player_bp))) 6e+02)
    (CallFunction|SetAirControl true)))

(fn ConstructionScript)