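; BP_StaticBlocks is a non-simulated block with a configurable mesh that acts as a bounce pad when its material is red.
; On hit it accepts the first-person character or a BP_Cube, then checks its material; non-red counts as Yellow, which does nothing.
; Bounce launches the player with a sound if their reflected velocity is zero, otherwise pushes the stored cube.
; Block rotation selects straight or angled launch vectors for both.
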(event OnComponentHit(Cube)
  (params (HitComponent :type Primitive%20Component%20Object%20Reference) (OtherActor :type Actor%20Object%20Reference) (OtherComp :type Primitive%20Component%20Object%20Reference) (NormalImpulse :type Vector :default "0, 0, 0") (Hit :type Hit%20Result%20Structure%20%28by%20ref%29))
  (Variables|Default|SetActor OtherActor)
  (Variables|Default|SetImpact%20vector (.impactnormal Hit))
  (bind _asbp_first_person_character (Utilities|Casting|CastToBP_FirstPersonCharacter (Variables|Default|GetActor))
    (:then
      (Variables|Default|SetPlayerRef _asbp_first_person_character))
    (:CastFailed
      (bind _asbp_cube (Utilities|Casting|CastToBP_Cube (Variables|Default|GetActor)))
      (Variables|Default|SetCubeREF _asbp_cube)))
  (bind _material (CallFunction|DetectColour))
  (if (Utilities|Enum|Equal(Enum) _material "Red")
    (CallFunction|Bounce (Variables|Default|GetActor))
    (elif (Utilities|Enum|Equal(Enum) _material "Yellow")
      _)))

(event EventBeginPlay
  (Physics|SetSimulatePhysics (Variables|Default|GetCube) false))

(fn ConstructionScript
  (Components|StaticMesh|SetStaticMesh (Variables|Default|GetCube) (Variables|Default|GetDesiredObject))
  (Rendering|Material|SetMaterial (Variables|Default|GetCube) 0 "/Game/Materials/M_BaseColour.M_BaseColour"))

(fn Bounce
  (params (ActorVelocity :type Actor%20Object%20Reference))
  (bind _cube (Variables|Default|GetCube))
  (bind _cube_2 (Variables|Default|GetCube))
  (bind _returnvalue (Transformation|GetWorldRotation _cube))
  (bind _returnvalue_2 (Transformation|GetWorldRotation _cube_2))
  (bind _returnvalue_3 (Utilities|Operators|EqualEqual :A _returnvalue))
  (if (and (== ActorVelocity (Variables|Default|GetPlayerRef)) (Utilities|Operators|EqualEqual :A (Math|Vector|GetReflectionVector (Transformation|GetVelocity) (Variables|Default|GetImpact%20vector))))
    (Development|PrintString "Hello")
    (if (not _returnvalue_3)
      (Audio|PlaySoundatLocation 0 "0, 0, 0" "0, 0, 0" 1.0 1.0 0.0 0 0 0 0)
      (bind _launchvec (CallFunction|CalculateLaunchVector))
      (Character|LaunchCharacter (Variables|Default|GetPlayerRef) _launchvec false false)
      (else
        (Audio|PlaySoundatLocation 0 "0, 0, 0" "0, 0, 0" 1.0 1.0 0.0 0 0 0 0)
        (Variables|Default|SetLaunchStrength 1000)
        (Character|LaunchCharacter (Variables|Default|GetPlayerRef) (* (Variables|Default|GetLaunchVector) (Variables|Default|GetLaunchStrength)) false true)))
    (elif _returnvalue_3
      (Variables|Default|SetLaunchStrength 5000)
      (Variables|Default|SetCubeLaunchVector "0.000000,0.000000,1000.000000")
      (Physics|AddForce (Variables|/Game/Cube/BP_Cube.BP_Cube_C|GetStaticMesh (Variables|Default|GetCubeREF)) (* (Variables|Default|GetCubeLaunchVector) (Variables|Default|GetLaunchStrength)) "None" false)
      (else
        (Variables|Default|SetLaunchStrength 5000)
        (bind _output_get (Variables|Default|SetCubeLaunchVector (Math|Vector|MakeVector (Math|Trig|Cos(Degrees) (.roll _returnvalue_2)) (Math|Trig|Sin(Degrees) (.pitch _returnvalue_2)) 0.0)))
        (Physics|AddImpulse (Variables|/Game/Cube/BP_Cube.BP_Cube_C|GetStaticMesh (Variables|Default|GetCubeREF)) (* (* _output_get (Variables|Default|GetLaunchStrength)) -1) "None" false)))))

(fn DetectColour
  (if (== (Rendering|Material|GetMaterial (Variables|Default|GetCube) 0) "/Game/Materials/MI_Red.MI_Red")
    (return "Red")
    (else
      (return "Yellow"))))

(fn CalculateLaunchVector
  (Variables|Default|SetLaunchStrength 1000)
  (return (* (Variables|Default|GetLaunchStrength) (+ (* (Transformation|GetWorldRotation (Variables|Default|GetCube)) -5.0) (Variables|Default|GetLaunchVector)))))