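; BP_Wall1 is a procedural wall actor that tiles randomized panel meshes into a grid sized by Height and Length.
; The construction script adds a scaled static mesh component per cell, choosing among three WallTypes through chained RandomPanels probability rolls.
; Each panel gets a random quarter-turn rotation to break up repetition.
; Randomness is unseeded, so the layout changes whenever construction reruns; the event graph is empty.
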(event EventBeginPlay)

(event Collision|EventActorBeginOverlap
  (params (OtherActor :type Actor%20Object%20Reference)))

(event EventTick
  (params (DeltaSeconds :type Float%20%28single-precision%29)))

(fn ConstructionScript
  (bind _returnvalue (Math|Conversions|ToFloat(Integer) 1))
  (bind _panelscale (Variables|Default|GetPanelScale))
  (bind _panelscale_2 (Variables|Default|GetPanelScale))
  (bind _returnvalue_2 (Math|Random|RandomFloatinRange 0.0 _returnvalue))
  (Components|StaticMesh|SetStaticMesh (Variables|Default|GetWall) (Utilities|Array|Get(acopy) (Variables|Default|GetWallTypes) 1))
  (Transformation|SetRelativeScale3D (Variables|Default|GetWall) (Math|Vector|MakeVector _panelscale _panelscale _panelscale))
  (for _index (range 0 (Variables|Default|GetHeight))
    (for _index_2 (range 0 (Variables|Default|GetLength))
      (bind _returnvalue_3 (AddComponent|AddStaticMeshComponent false))
      (if (<= _returnvalue_2 (Utilities|Array|Get(acopy) (Variables|Default|GetRandomPanels)))
        (Variables|Default|SetRandomIndex 0)
        (elif (<= _returnvalue_2 (Utilities|Array|Get(acopy) (Variables|Default|GetRandomPanels) 1))
          (Variables|Default|SetRandomIndex 1)
          (else
            (Variables|Default|SetRandomIndex 2))))
      (Components|StaticMesh|SetStaticMesh _returnvalue_3 (Utilities|Array|Get(acopy) (Variables|Default|GetWallTypes) (Variables|Default|GetRandomIndex)))
      (Transformation|SetRelativeLocation _returnvalue_3 (Math|Vector|MakeVector (* _index_2 (Variables|Default|GetPanelScale) 200) 0.0 (* _index (Variables|Default|GetPanelScale) 200)) false false)
      (switch int (Math|Random|RandomIntegerinRange 0 3)
        (:0
          (Variables|Default|SetRandomRotation 0.0))
        (:1
          (Variables|Default|SetRandomRotation 9e+01))
        (:2
          (Variables|Default|SetRandomRotation 1.8e+02))
        (:3
          (Variables|Default|SetRandomRotation 2.7e+02)))
      (Transformation|SetRelativeRotation _returnvalue_3 (Math|Rotator|MakeRotator 9e+01 (Variables|Default|GetRandomRotation) 0.0) false false)
      (Transformation|SetRelativeScale3D _returnvalue_3 (Math|Vector|MakeVector _panelscale_2 _panelscale_2 _panelscale_2)))))