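; Modular box builder that assembles a room-sized cube of wall panels and a top slab for level building.
; The construction script spawns BP_Wall1 child actors for four sides and a BP_Floor1 for the top, sized by Length, Width, Height and PanelScale.
; The DoNotRender map skips individual faces, and no bottom is built.
; Tick prints every floor tile location as debug output; older inline panel-generation logic remains unconnected.
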(event EventBeginPlay)

(event Collision|EventActorBeginOverlap
  (params (OtherActor :type Actor%20Object%20Reference)))

(event EventTick
  (params (DeltaSeconds :type Float%20%28single-precision%29))
  (for _array_element (Variables|/Game/Floors/BP_Floor1.BP_Floor1_C|GetFloorTiles (Variables|Default|GetAs%20BP%20Floor%201))
    (Development|PrintString (Utilities|String|ToString(Vector) (Transformation|GetWorldLocation _array_element)))))

(fn ConstructionScript
  (bind _panelscale (Variables|Default|GetPanelScale))
  (bind _width (Variables|Default|GetWidth))
  (bind _panelscale_2 (Variables|Default|GetPanelScale))
  (bind _panelscale_3 (Variables|Default|GetPanelScale))
  (bind _panelscale_4 (Variables|Default|GetPanelScale))
  (if (.Value (Utilities|Map|Find (Variables|Default|GetDoNotRender) "Left Side"))
    _
    (else
      (CallFunction|CreateWall "0, 0, 0" "0, 0, 0" (Variables|Default|GetLength))))
  (if (.Value (Utilities|Map|Find (Variables|Default|GetDoNotRender) "Top"))
    _
    (else
      (CallFunction|CreateFloor)
      (Transformation|SetActorRelativeLocation (Variables|Default|GetAs%20BP%20Floor%201) (Math|Vector|MakeVector 0.0 (+ (* (+ (Variables|Default|GetWidth) 1) _panelscale -200) (* _panelscale 1e+02)) (+ (* (+ (Variables|Default|GetHeight) 0) _panelscale_4 200) (* _panelscale_4 1e+02))))))
  (if (.Value (Utilities|Map|Find (Variables|Default|GetDoNotRender) "Back Side"))
    _
    (else
      (CallFunction|CreateWall (Math|Vector|MakeVector (* (Variables|Default|GetPanelScale) -1e+02) (+ (* (+ _width 1) _panelscale_3 -200) (* _panelscale_3 1e+02)) 0.0) "0.000000,90.000000,0.000000" _width)))
  (if (.Value (Utilities|Map|Find (Variables|Default|GetDoNotRender) "Front Side"))
    _
    (else
      (CallFunction|CreateWall (Math|Vector|MakeVector (+ (* (+ (Variables|Default|GetLength) 0) _panelscale_2 200) (* _panelscale_2 1e+02)) (* (Variables|Default|GetPanelScale) -1e+02) 0.0) "0.000000,270.000000,0.000000" (Variables|Default|GetWidth))))
  (if (not (.Value (Utilities|Map|Find (Variables|Default|GetDoNotRender) "Right Side")))
    (CallFunction|CreateWall (Math|Vector|MakeVector (+ (* (+ (Variables|Default|GetLength) 0) (Variables|Default|GetPanelScale) 200) 0.0) (+ (* (+ (Variables|Default|GetWidth) 1) (Variables|Default|GetPanelScale) -200) 0.0) 0.0) "0.000000,180.000000,0.000000" (Variables|Default|GetLength))))

(fn CreateWall
  (params (StartPos :type Vector) (Rotation :type Rotator) (Length :type Integer))
  (bind _returnvalue (AddComponent|AddChildActorComponent false))
  (ChildActorComponent|SetChildActorClass _returnvalue "/Game/Wall/Wall1/BP_Wall1.BP_Wall1_C")
  (bind _asbp_wall_1 (Utilities|Casting|CastToBP_Wall1 (Variables|/Script/Engine.ChildActorComponent|GetChildActor _returnvalue)))
  (Default|CreateWalls _asbp_wall_1 Length (Variables|Default|GetHeight) (Variables|Default|GetPanelScale) (Transformation|GetWorldRotation (Variables|Default|GetDefaultSceneRoot)))
  (Transformation|SetActorRelativeLocation _asbp_wall_1 StartPos)
  (Transformation|SetActorRelativeRotation _asbp_wall_1 Rotation))

(fn CreateFloor
  (bind _returnvalue (AddComponent|AddChildActorComponent false))
  (ChildActorComponent|SetChildActorClass _returnvalue "/Game/Floors/BP_Floor1.BP_Floor1_C")
  (bind _asbp_floor_1 (Utilities|Casting|CastToBP_Floor1 (Variables|/Script/Engine.ChildActorComponent|GetChildActor _returnvalue))
    (:then
      (Variables|Default|SetAs%20BP%20Floor%201 _asbp_floor_1)
      (Default|CreateFloor _asbp_floor_1 (Variables|Default|GetLength) (Variables|Default|GetWidth) (Variables|Default|GetPanelScale))
      (Transformation|SetActorRelativeRotation _asbp_floor_1 "0.000000,0.000000,0.000000"))
    (:CastFailed
      (Rendering|SetVisibility (Variables|Default|GetSphere) true false))))