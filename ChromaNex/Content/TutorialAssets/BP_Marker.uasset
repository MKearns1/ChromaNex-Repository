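; BP_Marker is a tutorial objective tracker that updates the objective text shown in the player's tutorial UI.
; On BeginPlay it caches the first-person character, then polls every Tick.
; While the objective is unmet, it writes the player's HasGun flag into the first array slot and clears that flag.
; A met objective advances the index, and a DoOnce gates ChangeObjective, which sets the indexed text.
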(event Custom|CheckFristObj
  (bind _playerref (Variables|Default|GetPlayerREF))
  (bind _hasgun (Variables|/Game/FirstPerson/Blueprints/BP_FirstPersonCharacter.BP_FirstPersonCharacter_C|GetHasGun _playerref))
  (if _hasgun
    (Utilities|Array|SetArrayElem (Variables|Default|GetObjectivesArray) 0 _hasgun true)
    (Variables|Default|SetObjective (Utilities|Array|Get(acopy) (Variables|Default|GetObjectivesArray)))))

(event EventBeginPlay
  (bind _asbp_first_person_character (Utilities|Casting|CastToBP_FirstPersonCharacter (Game|GetPlayerCharacter 0)))
  (Variables|Default|SetPlayerREF _asbp_first_person_character))

(event EventTick
  (params (DeltaSeconds :type Float%20%28single-precision%29))
  (if (Variables|Default|GetObjective)
    (bind _result (Math|Integer|IncrementInt (Variables|Default|GetObjectiveIndex))
      (:%20%20
        (Variables|Default|SetObjectiveIndex _result)
        (Variables|Default|SetObjective (Utilities|Array|Get(acopy) (Variables|Default|GetObjectivesArray) (Variables|Default|GetObjectiveIndex)))
        (goto _label Reset)))
    (else
      (CallFunction|CheckFristObj)
      (Variables|/Game/FirstPerson/Blueprints/BP_FirstPersonCharacter.BP_FirstPersonCharacter_C|SetHasGun (Variables|Default|GetPlayerREF) false)
      (Utilities|FlowControl|DoOnce false :!label _label
        (:Completed
          ;[1 1 1] Comment
          (Variables|Default|SetTutorialObjectives (Variables|/Game/FirstPerson/Blueprints/BP_FirstPersonCharacter.BP_FirstPersonCharacter_C|GetTutorialREF (Variables|Default|GetPlayerREF)))
          (CallFunction|ChangeObjective))))))

(fn ConstructionScript)

(fn ChangeObjective
  (Variables|/Script/UMG.TextBlock|SetText (Variables|/Game/TutorialAssets/Tutorial.Tutorial_C|GetObjectiveText (Variables|Default|GetTutorialObjectives)) (Utilities|Array|Get(acopy) (Variables|Default|GetObjectiveText) (Variables|Default|GetObjectiveIndex))))